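; BP_BYPlayerPawn is a player pawn Blueprint that handles montage animations for idle, shooting and death.
; Animation events play the idle montage, a single or burst pistol shot, or one of four death montages chosen by index.
; When a death montage completes, the skeletal mesh play rate drops to zero to freeze animation, and the idle event restores it.
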(event `self.OnPlayIdleAnimation`
  (bind _skeletalmesh (`self.SkeletalMesh`))
  (`SkeletalMeshComponent.SetPlayRate` _skeletalmesh 1.0)
  (`|PlayMontage` _skeletalmesh "/Game/Animation/AM_Idle.AM_Idle"))

(event `self.OnPlayShootAnimation`
  (params (bIsBurst :type Boolean))
  (if bIsBurst
    (`|PlayMontage` (`self.SkeletalMesh`) "/Game/Animation/AM_Pistol_Shoot_Burst.AM_Pistol_Shoot_Burst")
    (else
      (`|PlayMontage` (`self.SkeletalMesh`) "/Game/Animation/AM_Pistol_Shoot.AM_Pistol_Shoot"))))

(event `self.OnPlayDieAnimation`
  (params (Index :type Integer))
  (`|PlayMontage` (`self.SkeletalMesh`) (select `int` Index :`0` "/Game/Animation/AM_Die1.AM_Die1" :`1` "/Game/Animation/AM_Die2.AM_Die2" :`2` "/Game/Animation/AM_Die3.AM_Die3" :`3` "/Game/Animation/AM_Die4.AM_Die4" :!type "AnimMontage Object Reference")
    (:`OnCompleted`
      (`SkeletalMeshComponent.SetPlayRate` (`self.SkeletalMesh`) 0.0))))

(fn `UserConstructionScript`)